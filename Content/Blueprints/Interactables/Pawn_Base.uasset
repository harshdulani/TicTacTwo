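; Base pawn for a tic-tac-toe piece that is possessed, carried with the mouse and dropped onto grid boxes.
; While possessed, it spring-follows the deprojected cursor, and overlapped Grid_Selectable boxes check move validity against its value.
; Fire unpossesses it, springing to the box center or back to its start.
; A valid move updates TTTGameMode's grid, hides pawns already on that box, checks for a win and increments the move count.
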(event EventUnpossessed
  (params (OldController :type Controller%20Object%20Reference))
  (bind _returnvalue (Game|GetPlayerController 0))
  (Variables|CarryingPawn|SetshouldCarryWithMouse false)
  (Input|DisableInput _returnvalue)
  (bind _astttcontroller (Utilities|Casting|CastToTTTController _returnvalue))
  (Variables|/Game/Blueprints/Game/TTTController.TTTController_C|SetisCarryingPawn _astttcontroller false))

(event Collision|EventActorBeginOverlap
  (params (OtherActor :type Actor%20Object%20Reference))
  (bind _overlappedbox (Variables|MakingAMove|GetoverlappedBox))
  (bind _returnvalue (Utilities|Array|LastIndex _overlappedbox))
  ;[1 1 1] Hover over pieces and check if a valid move
  (if (== (Utilities|GetClass OtherActor) "/Game/Blueprints/Interactables/Grid_Selectable.Grid_Selectable_C")
    (Utilities|Array|SetArrayElem _overlappedbox (+ _returnvalue 1) OtherActor true)
    (bind _asgrid_selectable (Utilities|Casting|CastToGrid_Selectable (Utilities|Array|Get(acopy) _overlappedbox _returnvalue)))
    (bind _iscompatible (Default|CheckCompat _asgrid_selectable (Variables|MakingaMove|GetmyValue)))
    (Variables|MakingaMove|SetisMoveAllowed _iscompatible)
    (Variables|MakingaMove|SetmoveGridIndex (Variables|/Game/Blueprints/Interactables/Grid_Selectable.Grid_Selectable_C|GetmyIndex _asgrid_selectable))))

(event EventTick
  (params (DeltaSeconds :type Float%20%28single-precision%29))
  (if (Variables|CarryingPawn|GetshouldCarryWithMouse)
    ;[1 1 1] Carry Pawn With mouse
    (CallFunction|CarryPawn)
    (else
      ;[1 1 1] Post move lerping to grid box center
      (if (Math|Vector|NotEqual(Vector) (Variables|MakingAMove|GetfinalLerpToLocation) "0, 0, 0" 0.0001)
        (CallFunction|AutoLerptoLoc)))))

(event Collision|EventActorEndOverlap
  (params (OtherActor :type Actor%20Object%20Reference))
  ;[1 1 1] Hover over pieces and check if a valid move
  (if (== "/Game/Blueprints/Interactables/Grid_Selectable.Grid_Selectable_C" (Utilities|GetClass OtherActor))
    (Utilities|Array|RemoveItem (Variables|MakingAMove|GetoverlappedBox) OtherActor)))

(event EventBeginPlay
  ;[1 1 1] Start()
  (Variables|CarryingPawn|SetintialLocation (Transformation|GetWorldLocation (Variables|Default|GetScene))))

(event EventPossessed
  (params (NewController :type Controller%20Object%20Reference))
  (bind _returnvalue (Game|GetPlayerController 0))
  (Variables|CarryingPawn|SetshouldCarryWithMouse true)
  (Input|EnableInput _returnvalue)
  (bind _astttcontroller (Utilities|Casting|CastToTTTController _returnvalue))
  (Variables|/Game/Blueprints/Game/TTTController.TTTController_C|SetisCarryingPawn _astttcontroller true))

(event Input|ActionEvents|InputActionFire
  (params (Key :type Key%20Structure :default "None"))
  (bind _overlappedbox (Variables|MakingAMove|GetoverlappedBox))
  ;[1 1 1] handle selection and deselection of pawn
  (:Pressed
    (if (Variables|MakingaMove|GetisMoveAllowed)
      (bind _asgrid_selectable (Utilities|Casting|CastToGrid_Selectable (Utilities|Array|Get(acopy) _overlappedbox (Utilities|Array|LastIndex _overlappedbox))))
      (if (== (Variables|/Game/Blueprints/Interactables/Grid_Selectable.Grid_Selectable_C|GetmyIndex _asgrid_selectable) (Variables|MakingaMove|GetmoveGridIndex))
        (Variables|MakingAMove|SetfinalLerpToLocation (Transformation|GetActorLocation _asgrid_selectable))
        (CallFunction|MakeMove)
        (else
          (Variables|MakingAMove|SetfinalLerpToLocation (Variables|CarryingPawn|GetintialLocation) :!label _label)))
      (Pawn|UnPossess (Game|GetPlayerController 0))
      (elif (Variables|CarryingPawn|GetshouldCarryWithMouse)
        (goto _label)))))

(fn ConstructionScript)

(fn MakeMove
  (bind _astttgame_mode (Utilities|Casting|CastToTTTGameMode (Game|GetGameMode)))
  (Utilities|FlowControl|Sequence
    (:then_0
      ;[1 1 1] set grid index
      (if (> (Variables|MakingaMove|GetmoveGridIndex) -1)
        (Utilities|Array|SetArrayElem (Variables|/Game/Blueprints/Game/TTTGameMode.TTTGameMode_C|GetGridInfo _astttgame_mode) (Variables|MakingaMove|GetmoveGridIndex) (Variables|MakingaMove|GetmyValue) true)
        (else
          (return))))
    (:then_1
      ;[1 1 1] lerp to selection center, making a move and carrying this pawn shouldnt happen
      (Variables|MakingaMove|SetshouldPostMoveLerp true)
      (Variables|CarryingPawn|SetshouldCarryWithMouse false)
      (Variables|MakingaMove|SetisMoveAllowed false))
    (:then_2
      ;[1 1 1] turn visibility off, for any older pawns present there
      (bind _outactors (Actor|GetAllActorsOfClass "Pawn_Base_C"))
      (for _array_element _outactors
        (if (Math|Vector|Equal(Vector) (Transformation|GetWorldLocation (Variables|Pawn_Base_C|GetScene _array_element)) (Variables|MakingAMove|GetfinalLerpToLocation) 0.001)
          (Rendering|SetVisibility (Variables|Pawn_Base_C|GetStaticMesh _array_element) false false))))
    (:then_3
      ;[1 1 1] determine whether game is over or no
      (bind _astttgame_mode_2 (Utilities|Casting|CastToTTTGameMode (Game|GetGameMode)))
      (bind _result (Default|DidThisMoveWin _astttgame_mode_2 (Variables|MakingaMove|GetmoveGridIndex)))
      (Variables|MakingaMove|SetmoveGridIndex -1)
      (Default|IncreaseMoveCount _astttgame_mode_2))))

(fn CarryPawn
  (bind _returnvalue (Game|GetPlayerController 0))
  (bind _scene (Variables|Default|GetScene))
  (bind (_worldlocation _worlddirection) (Game|Player|ConvertMouseLocationToWorldSpace _returnvalue))
  (bind _output_get (Variables|CarryingPawn|SetcurrentLerpToLocation (+ _worldlocation (* (* _worlddirection (/ (.Z (Math|Vector|BreakVector _worldlocation)) (.Z (Math|Vector|BreakVector _worlddirection)))) -1))))
  (bind _returnvalue_2 (Class|KismetMathLibrary|VectorSpringInterp (Transformation|GetWorldLocation _scene) _output_get (Variables|CarryingPawn|GetSpring%20State) 0.75 0.75 0.1 1.0))
  (Transformation|SetWorldLocation _scene _returnvalue_2 false false))

(fn AutoLerptoLoc
  (bind _scene (Variables|Default|GetScene))
  (bind _returnvalue (Class|KismetMathLibrary|VectorSpringInterp (Transformation|GetWorldLocation _scene) (Variables|MakingAMove|GetfinalLerpToLocation) (Variables|CarryingPawn|GetSpring%20State) 0.75 0.75 0.1 1.0))
  (Transformation|SetWorldLocation _scene _returnvalue false false))