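; Selectable grid cell for what appears to be a tic-tac-toe variant (TTT), which validates and visually flags attempted moves.
; CheckCompat reads its MyIndex entry in the game mode's GridInfo, where sign and magnitude describe the occupying piece.
; A move passes if the cell is empty or the input has a different sign and larger magnitude.
; The mesh flashes green or red glass, then a timer restores clear glass.
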(fn ConstructionScript)

(fn CheckCompat
  (params (inputValue :type Integer))
  ;[1 1 1] if it is occupied by X = -1, 0 = 1. Not occupied = 0
  (bind _astttgame_mode (Utilities|Casting|CastToTTTGameMode (Game|GetGameMode)))
  (if (== (Utilities|Array|Get(acopy) (Variables|/Game/Blueprints/Game/TTTGameMode.TTTGameMode_C|GetGridInfo _astttgame_mode) (Variables|Default|GetmyIndex)) 0)
    _
    (elif (and (!= (Class|KismetMathLibrary|SignOfInteger inputValue) (Class|KismetMathLibrary|SignOfInteger (Utilities|Array|Get(acopy) (Variables|/Game/Blueprints/Game/TTTGameMode.TTTGameMode_C|GetGridInfo _astttgame_mode) (Variables|Default|GetmyIndex)))) (> (Math|Integer|Absolute(Integer) inputValue) (Math|Integer|Absolute(Integer) (Utilities|Array|Get(acopy) (Variables|/Game/Blueprints/Game/TTTGameMode.TTTGameMode_C|GetGridInfo _astttgame_mode) (Variables|Default|GetmyIndex)))))
      _
      (else
        (CallFunction|TurnRed)
        (return false))))
  (CallFunction|TurnGreen)
  (return true))

(fn TurnGreen
  (Rendering|Material|SetMaterial (Variables|Default|GetStaticMesh) 0 "/Game/Materials/M_GreenGlass.M_GreenGlass")
  (Utilities|Time|SetTimerbyFunctionName 0 "TurnTransparent" (Variables|Default|GetcolorTimer))
  (return))

(fn TurnRed
  (Rendering|Material|SetMaterial (Variables|Default|GetStaticMesh) 0 "/Game/Materials/M_RedGlass.M_RedGlass")
  (Utilities|Time|SetTimerbyFunctionName 0 "TurnTransparent" (Variables|Default|GetcolorTimer))
  (return))

(fn TurnTransparent
  (Rendering|Material|SetMaterial (Variables|Default|GetStaticMesh) 0 "/Game/StarterContent/Materials/M_Glass.M_Glass"))