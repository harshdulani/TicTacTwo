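; Game mode for tic-tac-toe that holds the grid state and move count and detects winning moves.
; DidThisMoveWin uses modulo math on the move index to test its row and column, plus both diagonals for even indices, and triggers game end on a win.
; MoveCheck treats three cells with the same sign, not all zero, as a line.
; IncreaseMoveCount counts moves and calls TogglePossessed on the player controller.
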(fn ConstructionScript)

(fn DidThisMoveWin
  (params (moveIndex :type Integer))
  (bind _returnvalue (Math|Integer|%(Integer) moveIndex 3))
  (bind _returnvalue_2 (- moveIndex _returnvalue))
  (bind _astttgame_mode (Utilities|Casting|CastToTTTGameMode (Game|GetGameMode)))
  (Utilities|FlowControl|Sequence
    (:then_0
      ;[1 1 1] Cannot win if atleast 3 moves are not made
      (if (< (Variables|Default|GettotalMovesMade) 3)
        (return false)))
    (:then_1
      ;[1 1 1] test patterns in %3 prove horizontal rows
      (bind _result (GameRules|MoveCheck (Utilities|Array|Get(acopy) (Variables|TTTGameMode_C|GetGridInfo _astttgame_mode) _returnvalue_2) (Utilities|Array|Get(acopy) (Variables|TTTGameMode_C|GetGridInfo _astttgame_mode) (+ _returnvalue_2 1)) (Utilities|Array|Get(acopy) (Variables|TTTGameMode_C|GetGridInfo _astttgame_mode) (+ _returnvalue_2 2))))
      (if _result
        (Default|CallGameEnd :!label _label)
        (return true)))
    (:then_2
      ;[1 1 1] x = i%3. arr[x], arr[x + 3], arr[x + 6] should have same values for column win case check
      (bind _result_2 (GameRules|MoveCheck (Utilities|Array|Get(acopy) (Variables|TTTGameMode_C|GetGridInfo _astttgame_mode) _returnvalue) (Utilities|Array|Get(acopy) (Variables|TTTGameMode_C|GetGridInfo _astttgame_mode) (+ _returnvalue 3)) (Utilities|Array|Get(acopy) (Variables|TTTGameMode_C|GetGridInfo _astttgame_mode) (+ _returnvalue 6))))
      (if _result_2
        (goto _label)))
    (:then_3
      ;[1 1 1] all indices that require diagonal checks lie on even nos.
      (if (== (Math|Integer|%(Integer) moveIndex 2) 0)
        (bind _result_3 (GameRules|MoveCheck (Utilities|Array|Get(acopy) (Variables|TTTGameMode_C|GetGridInfo _astttgame_mode)) (Utilities|Array|Get(acopy) (Variables|TTTGameMode_C|GetGridInfo _astttgame_mode) 4) (Utilities|Array|Get(acopy) (Variables|TTTGameMode_C|GetGridInfo _astttgame_mode) 8)))
        (if _result_3
          (goto _label)
          (else
            (bind _result_4 (GameRules|MoveCheck (Utilities|Array|Get(acopy) (Variables|TTTGameMode_C|GetGridInfo _astttgame_mode) 2) (Utilities|Array|Get(acopy) (Variables|TTTGameMode_C|GetGridInfo _astttgame_mode) 4) (Utilities|Array|Get(acopy) (Variables|TTTGameMode_C|GetGridInfo _astttgame_mode) 6)))
            (if _result_4
              (goto _label))))))
    (:then_4
      (return false))))

(fn IncreaseMoveCount
  (Variables|Default|SettotalMovesMade (+ (Variables|Default|GettotalMovesMade) 1))
  (bind _astttcontroller (Utilities|Casting|CastToTTTController (Game|GetPlayerController 0)))
  (Default|TogglePossessed _astttcontroller)
  (return))

(fn MoveCheck
  (params (n1 :type Integer) (n2 :type Integer) (n3 :type Integer))
  (bind _returnvalue (Class|KismetMathLibrary|SignOfInteger n2))
  (if (Math|Boolean|ANDBoolean (== n1 0) (== n2 0) (== n3 0))
    (return false)
    (elif (and (== (Class|KismetMathLibrary|SignOfInteger n1) _returnvalue) (== _returnvalue (Class|KismetMathLibrary|SignOfInteger n3)))
      (return true))))