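; Player controller for a two-sided pawn game (X and O) that decides which pawn the player possesses, tracked by PossessedSign.
; Fire, when not carrying a pawn, traces from the camera through the mouse to the Z=0 plane and possesses a hit Pawn_Base whose value sign matches.
; ChoosePossessed lets pawns offer themselves, defaulting to -1 while unset.
; TogglePossessed flips the sign and broadcasts PossessionToggled.
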(event EventTick
  (params (DeltaSeconds :type Float%20%28single-precision%29)))

(event Input|ActionEvents|InputActionFire
  (params (Key :type Key%20Structure :default "None"))
  (bind _returnvalue (Game|GetPlayerController 0))
  (bind (_worldlocation _worlddirection) (Game|Player|ConvertMouseLocationToWorldSpace _returnvalue))
  (:Pressed
    (if (not (Variables|Default|GetisCarryingPawn))
      (bind _outhit (Collision|LineTraceByChannel (Camera|GetCameraLocation (Variables|/Script/Engine.PlayerController|GetPlayerCameraManager _returnvalue)) (+ _worldlocation (* (* _worlddirection (/ (.Z (Math|Vector|BreakVector _worldlocation)) (.Z (Math|Vector|BreakVector _worlddirection)))) -1)) "TraceTypeQuery1" false 0 "ForDuration"))
      (if (== (Utilities|GetClass (.HitActor (Collision|BreakHitResult _outhit))) "/Game/Blueprints/Interactables/Pawn_X.Pawn_X_C")
        (bind _aspawn_base (Utilities|Casting|CastToPawn_Base (.HitActor (Collision|BreakHitResult _outhit)) :!label _label))
        (if (== (Class|KismetMathLibrary|SignOfInteger (Variables|/Game/Blueprints/Interactables/Pawn_Base.Pawn_Base_C|GetmyValue _aspawn_base)) (Variables|Default|GetpossessedSign))
          (Pawn|Possess _aspawn_base))
        (elif (== (Utilities|GetClass (.HitActor (Collision|BreakHitResult _outhit))) (Utilities|GetClass (.HitActor (Collision|BreakHitResult _outhit))))
          (goto _label))))))

(fn ConstructionScript)

(fn ChoosePossessed
  (params (candidateValue :type Integer) (pawnReference :type Pawn%20Base%20Object%20Reference))
  ;[1 1 1] Since it's going to be called by both the pawns, the need for checking their values, and if required their refs
  (if (== candidateValue (Variables|Default|GetpossessedSign))
    (Pawn|Possess pawnReference :!label _label)
    (Variables|Default|SetpossessedSign candidateValue)
    (elif (and (== (Variables|Default|GetpossessedSign) 0) (== candidateValue -1))
      (goto _label))))

(fn TogglePossessed
  ;[1 1 1] Toggle desired Possessed between X & 0
  (bind _output_get (Variables|Default|SetpossessedSign (* (Variables|Default|GetpossessedSign) -1)))
  (Default|CallPossessionToggled (Variables|Default|GetpossessedSign))
  (return _output_get))